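; Cat Blueprint that extends its parent's directional push mechanic with force UI and push state flags, and pauses the game on the Pause key.
; Forward, right and left push starts call the parent, then show a Force_UI widget if LoadingForce is set.
; ReleaseSelected calls the parent and removes that widget.
; Push raises the flag matching PushDirectionMode for half a second, then clears it.
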(event `Key|Pause`
  (params (Key :type "Key Structure"))
  (:`Pressed`
    (`GameplayStatics.SetGamePaused` true)))

(event `self.StartPushForward`
  (`parent.StartPushForward`)
  (if (`self.LoadingForce`)
    (bind _returnvalue (`|CreateWidget` "/Game/Blueprints/UI/Force_UI.Force_UI_C"))
    (`UserWidget.AddToViewport` _returnvalue 0)
    (set `self.Force WIdget` _returnvalue)))

(event `self.StartPushRight`
  (`parent.StartPushRight`)
  (if (`self.LoadingForce`)
    (bind _returnvalue (`|CreateWidget` "/Game/Blueprints/UI/Force_UI.Force_UI_C"))
    (`UserWidget.AddToViewport` _returnvalue 0)
    (set `self.Force WIdget` _returnvalue)))

(event `self.StartPushLeft`
  (`parent.StartPushLeft`)
  (if (`self.LoadingForce`)
    (bind _returnvalue (`|CreateWidget` "/Game/Blueprints/UI/Force_UI.Force_UI_C"))
    (`UserWidget.AddToViewport` _returnvalue 0)
    (set `self.Force WIdget` _returnvalue)))

(event `self.ReleaseSelected`
  (`parent.ReleaseSelected`)
  (if (`KismetSystemLibrary.IsValid` (`self.Force WIdget`))
    (`Widget.RemoveFromParent` (`self.Force WIdget`))))

(event `self.Push`
  (switch `string` (`self.PushDirectionMode`)
    (:`Forward`
      (set `self.IsPushingForward` true)
      (`KismetSystemLibrary.Delay` 0.5)
      (set `self.IsPushingForward` false))
    (:`Right`
      (set `self.IsPushingRight` true)
      (`KismetSystemLibrary.Delay` 0.5)
      (set `self.IsPushingRight` false))
    (:`Left`
      (set `self.IsPushingLeft` true)
      (`KismetSystemLibrary.Delay` 0.5)
      (set `self.IsPushingLeft` false))))

(fn `UserConstructionScript`)