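; Presentation actor that displays a cat lying down in a looping animation, showing the breed currently stored in the game instance.
; On BeginPlay it plays the lying loop on its skeletal mesh without setting a breed.
; The UpdateCatRace event reads CatRace from GameInstance_BP, swaps in the matching breed mesh with pose reinit, then restarts the loop.
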(event `self.ReceiveBeginPlay`
  (`SkeletalMeshComponent.PlayAnimation` (`self.SkeletalMeshComponent`) "/Game/LowPoly_Cat/Animations/Anim_Cat_Lie_loop.Anim_Cat_Lie_loop" true))

(event `Update Cat Race`
  (bind _asgame_instance_bp (cast `/Game/Blueprints/GameInstance_BP` (`GameplayStatics.GetGameInstance`)))
  (switch `/Game/Cats_Enum` (`/Game/Blueprints/GameInstance_BP.CatRace` _asgame_instance_bp)
    (:`NewEnumerator0`
      (`SkinnedMeshComponent.SetSkinnedAssetAndUpdate` (`self.SkeletalMeshComponent`) "/Game/LowPoly_Cat/Meshes/Mesh_Cat_Abyss.Mesh_Cat_Abyss" true))
    (:`NewEnumerator1`
      (`SkinnedMeshComponent.SetSkinnedAssetAndUpdate` (`self.SkeletalMeshComponent`) "/Game/LowPoly_Cat/Meshes/Mesh_Cat_black.Mesh_Cat_black" true))
    (:`NewEnumerator2`
      (`SkinnedMeshComponent.SetSkinnedAssetAndUpdate` (`self.SkeletalMeshComponent`) "/Game/LowPoly_Cat/Meshes/Mesh_Cat_Black_White.Mesh_Cat_Black_White" true))
    (:`NewEnumerator3`
      (`SkinnedMeshComponent.SetSkinnedAssetAndUpdate` (`self.SkeletalMeshComponent`) "/Game/LowPoly_Cat/Meshes/Mesh_Cat_Blue.Mesh_Cat_Blue" true))
    (:`NewEnumerator4`
      (`SkinnedMeshComponent.SetSkinnedAssetAndUpdate` (`self.SkeletalMeshComponent`) "/Game/LowPoly_Cat/Meshes/Mesh_Cat_Bobtail.Mesh_Cat_Bobtail" true))
    (:`NewEnumerator5`
      (`SkinnedMeshComponent.SetSkinnedAssetAndUpdate` (`self.SkeletalMeshComponent`) "/Game/LowPoly_Cat/Meshes/Mesh_Cat_Brit.Mesh_Cat_Brit" true))
    (:`NewEnumerator6`
      (`SkinnedMeshComponent.SetSkinnedAssetAndUpdate` (`self.SkeletalMeshComponent`) "/Game/LowPoly_Cat/Meshes/Mesh_Cat_brown.Mesh_Cat_brown" true))
    (:`NewEnumerator7`
      (`SkinnedMeshComponent.SetSkinnedAssetAndUpdate` (`self.SkeletalMeshComponent`) "/Game/LowPoly_Cat/Meshes/Mesh_Cat_maine.Mesh_Cat_maine" true))
    (:`NewEnumerator8`
      (`SkinnedMeshComponent.SetSkinnedAssetAndUpdate` (`self.SkeletalMeshComponent`) "/Game/LowPoly_Cat/Meshes/Mesh_Cat_Pers.Mesh_Cat_Pers" true))
    (:`NewEnumerator9`
      (`SkinnedMeshComponent.SetSkinnedAssetAndUpdate` (`self.SkeletalMeshComponent`) "/Game/LowPoly_Cat/Meshes/Mesh_Cat_Red.Mesh_Cat_Red" true))
    (:`NewEnumerator10`
      (`SkinnedMeshComponent.SetSkinnedAssetAndUpdate` (`self.SkeletalMeshComponent`) "/Game/LowPoly_Cat/Meshes/Mesh_Cat_Red_White.Mesh_Cat_Red_White" true))
    (:`NewEnumerator11`
      (`SkinnedMeshComponent.SetSkinnedAssetAndUpdate` (`self.SkeletalMeshComponent`) "/Game/LowPoly_Cat/Meshes/Mesh_Cat_Siamese.Mesh_Cat_Siamese" true))
    (:`NewEnumerator12`
      (`SkinnedMeshComponent.SetSkinnedAssetAndUpdate` (`self.SkeletalMeshComponent`) "/Game/LowPoly_Cat/Meshes/Mesh_Cat_Sphynx.Mesh_Cat_Sphynx" true))
    (:`NewEnumerator13`
      (`SkinnedMeshComponent.SetSkinnedAssetAndUpdate` (`self.SkeletalMeshComponent`) "/Game/LowPoly_Cat/Meshes/Mesh_Cat_white.Mesh_Cat_white" true)))
  (`SkeletalMeshComponent.PlayAnimation` (`self.SkeletalMeshComponent`) "/Game/LowPoly_Cat/Animations/Anim_Cat_Lie_loop.Anim_Cat_Lie_loop" true))

(fn `UserConstructionScript`)