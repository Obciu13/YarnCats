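; YarnsShelf_BP is a shelf that collects yarn items and ends the game when full.
; When a Yarn_BP overlaps its box, it destroys that actor, increments a counter and reveals the matching one of four yarn components.
; The fourth yarn also shows the GameCompleted widget, switches to UI-only input and displays the mouse cursor.
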(event `self.Box.OnComponentBeginOverlap`
  (params (OverlappedComponent :type "PrimitiveComponent Object Reference") (OtherActor :type "Actor Object Reference") (OtherComp :type "PrimitiveComponent Object Reference") (OtherBodyIndex :type Integer) (bFromSweep :type Boolean) (SweepResult :type "HitResult Structure (by ref)"))
  (bind _returnvalue (`GameplayStatics.GetPlayerController` 0))
  (bind _asyarn_bp (cast `/Game/Blueprints/Yarns/Yarn_BP` OtherActor))
  (bind _result (`/Engine/EditorBlueprintResources/StandardMacros.IncrementInt` (`self.YarnCounter`))
    (:`  `
      (`self.K2_DestroyActor` _asyarn_bp)
      (`KismetSystemLibrary.PrintString` (`KismetStringLibrary.Conv_IntToString` _result))
      (switch `int` _result
        (:`1`
          (`SceneComponent.SetVisibility` (`self.Yarn1`) true false))
        (:`2`
          (`SceneComponent.SetVisibility` (`self.Yarn2`) true false))
        (:`3`
          (`SceneComponent.SetVisibility` (`self.Yarn3`) true false))
        (:`4`
          (`SceneComponent.SetVisibility` (`self.Yarn4`) true false)
          (bind _returnvalue_2 (`|CreateWidget` "/Game/Blueprints/UI/GameCompleted.GameCompleted_C" _returnvalue))
          (`UserWidget.AddToViewport` _returnvalue_2 0)
          (`WidgetBlueprintLibrary.SetInputMode_UIOnlyEx` _returnvalue _returnvalue_2)
          (set `PlayerController.bShowMouseCursor` true _returnvalue))))))

(fn `UserConstructionScript`)